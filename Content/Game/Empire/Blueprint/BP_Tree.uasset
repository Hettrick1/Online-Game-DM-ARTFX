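; Harvestable tree that players chop for wood, with randomized yaw and scale, a harvest-percent widget and timed respawn.
; A box trigger registers one character at a time as harvester.
; Server-called TreeHarvestPercentage accumulates progress, then adds wood through GS_Empire and tells the character to disable tree collision.
; Externally triggered RotateTree starts a timeline fall on either axis, then timers chain shrinking and restoring rotation, size and collision.
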(event OnComponentBeginOverlap(Box)
  (params (OverlappedComponent :type Primitive%20Component%20Object%20Reference) (OtherActor :type Actor%20Object%20Reference) (OtherComp :type Primitive%20Component%20Object%20Reference) (OtherBodyIndex :type Integer) (bFromSweep :type Boolean) (SweepResult :type Hit%20Result%20Structure%20%28by%20ref%29))
  ;[1 1 1] On trigger enter / leave
  (Utilities|IsValid (Variables|Default|GetAs%20BP%20Third%20Person%20Character)
    (:Is%20Not%20Valid
      (CallFunction|SetCanHarvestWood OtherActor true))))

(event OnComponentEndOverlap(Box)
  (params (OverlappedComponent :type Primitive%20Component%20Object%20Reference) (OtherActor :type Actor%20Object%20Reference) (OtherComp :type Primitive%20Component%20Object%20Reference) (OtherBodyIndex :type Integer))
  ;[1 1 1] On trigger enter / leave
  (if (== OtherActor (Variables|Default|GetAs%20BP%20Third%20Person%20Character))
    (CallFunction|SetCanHarvestWood OtherActor false)
    (Variables|Default|SetharvestPercent 0.0)))

(event Custom|SetCanHarvestWood
  (params (actor :type Actor%20Object%20Reference) (bool :type Boolean))
  ;[1 1 1] Set player can harvest state
  (bind _asbp_third_person_character (Utilities|Casting|CastToBP_ThirdPersonCharacter actor))
  (Variables|Default|SetAs%20BP%20Third%20Person%20Character _asbp_third_person_character)
  (if bool
    (Default|SetCanHarvestTree _asbp_third_person_character true self)
    (else
      (Default|SetCanHarvestTree _asbp_third_person_character false)
      (Variables|Default|SetAs%20BP%20Third%20Person%20Character 0))))

(event Custom|TreeHarvestPercentage
  ;[1 1 1] Harvest tree and check if the harvest is finished
  (if (>= (Variables|Default|GetharvestPercent) 1e+02)
    (Development|PrintString "COUPE")
    (Variables|Default|SetharvestPercent 0.0)
    (Utilities|FlowControl|DelayUntilNextTick)
    (Default|SetCanHarvestTree (Variables|Default|GetAs%20BP%20Third%20Person%20Character) false)
    (CallFunction|HarvestTree) ; Increase wood inventory amount
    (Default|SetTreeCollisionState (Variables|Default|GetAs%20BP%20Third%20Person%20Character) self false)
    (else
      (Variables|Default|SetharvestPercent (+ (Variables|Default|GetharvestPercent) (* (Utilities|Time|GetWorldDeltaSeconds) 5e+01))))))

(event Custom|RotateWidget
  (params (Target :type Actor%20Object%20Reference))
  ;[1 1 1] Rotate the widget to be facing the owning player
  (Transformation|SetWorldRotation (Variables|Default|GetScene) (Math|Rotator|MakeRotator 0.0 0.0 (.yaw (Math|Rotator|FindLookatRotation (Transformation|GetWorldLocation (Variables|Default|GetScene)) (Transformation|GetActorLocation Target)))) false false))

(event Custom|HarvestTree
  ;[1 1 1] Update the wood amount in inventory
  (bind _asgs_empire (Utilities|Casting|CastToGS_Empire (Game|GetGameState)))
  (Default|UpdateWoodRep _asgs_empire 10))

(event Custom|RotateTree
  (params (axis :type Integer))
  (bind _cylinder (Variables|Default|GetCylinder))
  (bind _relativerotation (Variables|/Script/Engine.SceneComponent|GetRelativeRotation _cylinder))
  ;[1 1 1] Make te tree fall when harvested
  (bind _alpha (Timeline|TreeRotationLerp PlayFromStart) ; Tree fall animation
    (:Update
      (switch int axis
        (:0
          (Variables|Default|SetrelRotY (Math|Float|Lerp 0.0 9e+01 _alpha))
          (Variables|Default|SetrelRotX (.roll _relativerotation)))
        (:1
          (Variables|Default|SetrelRotX (Math|Float|Lerp 0.0 9e+01 _alpha))
          (Variables|Default|SetrelRotY (.pitch _relativerotation))))
      (Transformation|SetRelativeRotation (Variables|Default|GetCylinder) (Math|Rotator|MakeRotator (Variables|Default|GetrelRotX) (Variables|Default|GetrelRotY) (.yaw _relativerotation)) false true))
    (:Finished
      (Utilities|Time|SetTimerbyEvent (delegate Custom|DespawnTree) 1.0 false true))))

(event Custom|DespawnTree
  (bind _returnvalue (Transformation|GetActorScale3D))
  ;[1 1 1] Make te tree fall when harvested
  (bind _alpha (Timeline|SizeChangeLerp PlayFromStart) ; Despawn Animation
    (:Update
      (Transformation|SetActorScale3D (Math|Vector|MakeVector (Math|Float|Lerp (.x _returnvalue) 0.001 _alpha) (Math|Float|Lerp (.y _returnvalue) 0.001 _alpha) (Math|Float|Lerp (.z _returnvalue) 0.001 _alpha))))
    (:Finished
      (Utilities|Time|SetTimerbyEvent (delegate Custom|RespawnTree) 6.0 false true) ; Delay before Respawn
    )))

(event Custom|RespawnTree
  ;[1 1 1] Make te tree fall when harvested
  (Transformation|SetRelativeRotation (Variables|Default|GetCylinder) (Math|Rotator|MakeRotator 0.0 0.0 (.yaw (Variables|/Script/Engine.SceneComponent|GetRelativeRotation (Variables|Default|GetCylinder)))) false true)
  (Transformation|SetActorScale3D (Variables|Default|GetinitialSize))
  (Collision|SetActorEnableCollision true))

(event EventBeginPlay
  ;[1 1 1] Cast widget on the begin play
  (bind _aswbp_harvest_percent (Utilities|Casting|CastToWBP_HarvestPercent (UserInterface|GetWidget (Variables|Default|GetWidget))))
  (Variables|Default|SetharvestPercentWidget _aswbp_harvest_percent))

(fn ConstructionScript
  (bind _returnvalue (Math|Random|RandomFloatinRange 0.5 1.2))
  (bind _scene (Variables|Default|GetScene))
  ;[1 1 1] Random tree rotation
  (Transformation|SetRelativeRotation (Variables|Default|GetCylinder) (Math|Rotator|MakeRotator 0.0 0.0 (Math|Random|RandomFloatinRange 0.0 1.8e+02)) false false)
  (Transformation|SetActorScale3D (Math|Vector|MakeVector _returnvalue _returnvalue _returnvalue))
  (bind _output_get (Variables|Default|SetinitialSize (Transformation|GetActorScale3D)))
  (Transformation|SetRelativeScale3D (Variables|Default|GetWidget) (/ "1.000000,1.000000,1.000000" _output_get))
  (Transformation|SetWorldLocation _scene (+ (Transformation|GetWorldLocation _scene) "0.000000,0.000000,150.000000") false false))