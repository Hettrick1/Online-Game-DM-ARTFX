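; BP_Rock is a harvestable rock that adds stone to the GS_Empire game state and can respawn.
; Its overlap box lets one BP_ThirdPersonCharacter at a time harvest it.
; A server-side event raises harvest progress, then awards stone and has the character disable the rock's collision.
; A separate despawn event shrinks it by timeline, then a timer restores collision and its randomized construction-time scale.
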(event OnComponentBeginOverlap(Box)
  (params (OverlappedComponent :type Primitive%20Component%20Object%20Reference) (OtherActor :type Actor%20Object%20Reference) (OtherComp :type Primitive%20Component%20Object%20Reference) (OtherBodyIndex :type Integer) (bFromSweep :type Boolean) (SweepResult :type Hit%20Result%20Structure%20%28by%20ref%29))
  ;[1 1 1] On Trigger enter / leave
  (Utilities|IsValid (Variables|Default|GetAs%20BP%20Third%20Person%20Character)
    (:Is%20Not%20Valid
      (CallFunction|SetCanHarvestStone OtherActor true))))

(event OnComponentEndOverlap(Box)
  (params (OverlappedComponent :type Primitive%20Component%20Object%20Reference) (OtherActor :type Actor%20Object%20Reference) (OtherComp :type Primitive%20Component%20Object%20Reference) (OtherBodyIndex :type Integer))
  ;[1 1 1] On Trigger enter / leave
  (if (== OtherActor (Variables|Default|GetAs%20BP%20Third%20Person%20Character))
    (CallFunction|SetCanHarvestStone OtherActor false)
    (Variables|Default|SetharvestPercent 0.0)))

(event Custom|SetCanHarvestStone
  (params (Actor :type Actor%20Object%20Reference) (bool :type Boolean))
  ;[1 1 1] Set player can harvest state
  (bind _asbp_third_person_character (Utilities|Casting|CastToBP_ThirdPersonCharacter Actor))
  (Variables|Default|SetAs%20BP%20Third%20Person%20Character _asbp_third_person_character)
  (if bool
    (Default|SetCanHarvestRock (Variables|Default|GetAs%20BP%20Third%20Person%20Character) true self)
    (else
      (Default|SetCanHarvestRock (Variables|Default|GetAs%20BP%20Third%20Person%20Character) false)
      (Variables|Default|SetAs%20BP%20Third%20Person%20Character 0))))

(event Custom|RockHarvestPercentage
  ;[1 1 1] Harvest rock and check if the harvest is finished
  (Development|PrintString (Utilities|String|ToString(Float) (Variables|Default|GetharvestPercent)))
  (if (>= (Variables|Default|GetharvestPercent) 1e+02)
    (Development|PrintString "CASSE")
    (Variables|Default|SetharvestPercent 0.0)
    (Default|SetCanHarvestRock (Variables|Default|GetAs%20BP%20Third%20Person%20Character) false)
    (CallFunction|HarvestRock)
    (Default|SetRockCollisionState (Variables|Default|GetAs%20BP%20Third%20Person%20Character) self false)
    (else
      (Variables|Default|SetharvestPercent (+ (Variables|Default|GetharvestPercent) (* (Utilities|Time|GetWorldDeltaSeconds) 5e+01))))))

(event Custom|HarvestRock
  ;[1 1 1] Update the stone amount in the inventory
  (bind _asgs_empire (Utilities|Casting|CastToGS_Empire (Game|GetGameState)))
  (Default|UpdateStoneRep _asgs_empire 10))

(event Custom|DespawnRock
  (bind _returnvalue (Transformation|GetActorScale3D))
  ;[1 1 1] Despawn rock animation
  (bind _alpha (Timeline|SizeChangeLerp PlayFromStart) ; Despawn Animation
    (:Update
      (Transformation|SetActorScale3D (Math|Vector|MakeVector (Math|Float|Lerp (.x _returnvalue) 0.001 _alpha) (Math|Float|Lerp (.y _returnvalue) 0.001 _alpha) (Math|Float|Lerp (.z _returnvalue) 0.001 _alpha))))
    (:Finished
      (Utilities|Time|SetTimerbyEvent (delegate Custom|RespawnTree) 6.0 false true) ; Delay before Respawn
    )))

(event Custom|RespawnTree
  ;[1 1 1] Despawn rock animation
  (Transformation|SetActorScale3D (Variables|Default|GetinitialSize))
  (Collision|SetActorEnableCollision true))

(fn ConstructionScript
  (bind _returnvalue (Math|Random|RandomFloatinRange 0.5 1.2))
  (Transformation|SetActorRotation (Math|Rotator|MakeRotator 0.0 0.0 (Math|Random|RandomFloatinRange 0.0 1.8e+02)))
  (Transformation|SetActorScale3D (Math|Vector|MakeVector _returnvalue _returnvalue _returnvalue))
  (Variables|Default|SetinitialSize (Transformation|GetActorScale3D)))