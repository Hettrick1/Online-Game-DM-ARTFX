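; Buyable house plot that shows a buy-house widget to a player character entering its box.
; One tick after BeginPlay it box-traces WorldStatic objects at its bounds origin and destroys itself on a hit, intended to clear slots already holding a house.
; It tracks occupants, offers purchase to one character at a time, and rejects characters already holding a HouseSlot.
; Leaving hides the PC_Empire HUD's leave warning and the buyer's widget.
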(event OnComponentBeginOverlap(Box)
  (params (OverlappedComponent :type Primitive%20Component%20Object%20Reference) (OtherActor :type Actor%20Object%20Reference) (OtherComp :type Primitive%20Component%20Object%20Reference) (OtherBodyIndex :type Integer) (bFromSweep :type Boolean) (SweepResult :type Hit%20Result%20Structure%20%28by%20ref%29))
  ;[1 1 1] If overlap, show the buy widget. If leaving, set the leave warning to hidden
  (Utilities|Array|Add (Variables|Default|GetinActors) (.AsBP%20Third%20Person%20Character (Utilities|Casting|CastToBP_ThirdPersonCharacter OtherActor)))
  (Utilities|IsValid (Variables|Default|GetAs%20BP%20Third%20Person%20Character)
    (:Is%20Not%20Valid
      (CallFunction|BuyHouseWidget OtherActor true))))

(event OnComponentEndOverlap(Box)
  (params (OverlappedComponent :type Primitive%20Component%20Object%20Reference) (OtherActor :type Actor%20Object%20Reference) (OtherComp :type Primitive%20Component%20Object%20Reference) (OtherBodyIndex :type Integer))
  ;[1 1 1] If overlap, show the buy widget. If leaving, set the leave warning to hidden
  (for _array_element (Variables|Default|GetinActors)
    (if (== _array_element OtherActor)
      (bind _aspc_empire (Utilities|Casting|CastToPC_Empire (Pawn|GetController _array_element)))
      (Utilities|IsValid (Variables|/Game/Game/Empire/PC_Empire.PC_Empire_C|GetbaseHudRef _aspc_empire)
        (:Is%20Valid
          (Default|ChangeLeaveVisibility (Variables|/Game/Game/Empire/PC_Empire.PC_Empire_C|GetbaseHudRef _aspc_empire) false)
          (Utilities|Array|RemoveItem (Variables|Default|GetinActors) _array_element)))))
  (if (== OtherActor (Variables|Default|GetAs%20BP%20Third%20Person%20Character))
    (CallFunction|BuyHouseWidget OtherActor false)))

(event Custom|BuyHouseWidget
  (params (otherActor :type Actor%20Object%20Reference) (show :type Boolean))
  ;[1 1 1] Show/Hide buy house widget
  (bind _aspc_empire (Utilities|Casting|CastToPC_Empire (Game|GetInstigatorController otherActor)))
  (if show
    (bind _output_get (Variables|Default|SetAs%20BP%20Third%20Person%20Character (.AsBP%20Third%20Person%20Character (Utilities|Casting|CastToBP_ThirdPersonCharacter otherActor))))
    (Utilities|IsValid (Variables|/Game/ThirdPerson/Blueprints/BP_ThirdPersonCharacter.BP_ThirdPersonCharacter_C|GetHouse%20Slot _output_get)
      (:Is%20Valid
        (Variables|Default|SetAs%20BP%20Third%20Person%20Character 0)
        (Development|PrintString "YOU ARE ALREADY BUYING ANOTHER HOUSE"))
      (:Is%20Not%20Valid
        (Default|ShowBuyHouse _aspc_empire self)))
    (else
      (Default|HideBuyHouse _aspc_empire)
      (Variables|Default|SetAs%20BP%20Third%20Person%20Character 0))))

(event EventBeginPlay
  (bind _origin (Collision|GetActorBounds false false))
  ;[1 1 1] If there is a house at the begin play, destroy self
  (Utilities|FlowControl|DelayUntilNextTick)
  (bind _outhits (Class|KismetSystemLibrary|BoxTraceMultiforObjects _origin _origin "1.000000,1.000000,1.000000" "0, 0, 0" (Utilities|Array|MakeArray "ObjectTypeQuery1") false 0 "None" true))
  (for _array_element _outhits
    (Utilities|IsValid (.HitActor (Collision|BreakHitResult _array_element))
      (:Is%20Valid
        (Development|PrintString (Utilities|GetDisplayName (.HitActor (Collision|BreakHitResult _array_element))))
        (Actor|DestroyActor)))))

(fn ConstructionScript)