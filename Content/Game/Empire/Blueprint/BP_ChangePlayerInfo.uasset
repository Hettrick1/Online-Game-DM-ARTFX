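; BP_ChangePlayerInfo is a trigger zone that shows the player info setter widget while a player is inside it.
; Box begin and end overlap call show and hide events with the overlapping actor.
; Each event casts that actor's instigator controller to PC_Empire and calls ShowInfoSetterWidget or HideInfoSetterWidget, ignoring actors without such a controller.
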(event OnComponentBeginOverlap(Box)
  (params (OverlappedComponent :type Primitive%20Component%20Object%20Reference) (OtherActor :type Actor%20Object%20Reference) (OtherComp :type Primitive%20Component%20Object%20Reference) (OtherBodyIndex :type Integer) (bFromSweep :type Boolean) (SweepResult :type Hit%20Result%20Structure%20%28by%20ref%29))
  ;[1 1 1] Show / hide player info setter
  (CallFunction|ShowPlayerInfoSetter OtherActor))

(event OnComponentEndOverlap(Box)
  (params (OverlappedComponent :type Primitive%20Component%20Object%20Reference) (OtherActor :type Actor%20Object%20Reference) (OtherComp :type Primitive%20Component%20Object%20Reference) (OtherBodyIndex :type Integer))
  ;[1 1 1] Show / hide player info setter
  (CallFunction|HidePlayerInfoSetter OtherActor))

(event Custom|ShowPlayerInfoSetter
  (params (otherActor :type Actor%20Object%20Reference))
  ;[1 1 1] Show / hide player info setter
  (bind _aspc_empire (Utilities|Casting|CastToPC_Empire (Game|GetInstigatorController otherActor)))
  (Default|ShowInfoSetterWidget _aspc_empire))

(event Custom|HidePlayerInfoSetter
  (params (otherActor :type Actor%20Object%20Reference))
  ;[1 1 1] Show / hide player info setter
  (bind _aspc_empire (Utilities|Casting|CastToPC_Empire (Game|GetInstigatorController otherActor)))
  (Default|HideInfoSetterWidget _aspc_empire))

(fn ConstructionScript)