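; GM_Empire is a game mode that sets up each player on login.
; PostLogin calls InitializeSaveSystem on GI_Game, then spawns a BP_ThirdPersonCharacter at the PlayerStart selected by a running index and has the new player possess it.
; The index advances per login with no wraparound, and a failed game instance cast only prints an error, leaving that player without this spawn.
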(event EventPostLogin
  (params (NewPlayer :type Player%20Controller%20Object%20Reference))
  (bind _asgi_game (Utilities|Casting|CastToGI_Game (Game|GetGameInstance))
    (:then
      (Default|InitializeSaveSystem _asgi_game)
      (bind _outactors (Actor|GetAllActorsOfClass "/Script/Engine.PlayerStart"))
      (bind _returnvalue (Game|SpawnActorfromClass "/Game/ThirdPerson/Blueprints/BP_ThirdPersonCharacter.BP_ThirdPersonCharacter_C" (Math|Transform|MakeTransform (.location (Transformation|GetActorTransform (Utilities|Array|Get(acopy) _outactors (Variables|Default|Getindex)))) (.rotation (Transformation|GetActorTransform (Utilities|Array|Get(acopy) _outactors (Variables|Default|Getindex)))) "1.000000,1.000000,1.000000") "AdjustIfPossibleButAlwaysSpawn" "MultiplyWithRoot" 0 0))
      (Variables|Default|Setindex (+ (Variables|Default|Getindex) 1))
      (Pawn|Possess NewPlayer _returnvalue))
    (:CastFailed
      (Development|PrintString "Fail to cast to GI"))))

(fn ConstructionScript)