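; Player controller for the Empire game that manages the local player's HUD, buy-house widget and player info setter widget.
; BeginPlay adds the base HUD, and show/hide events create or remove each menu while tracking which is open.
; The buy-house events also pass or clear the house slot on the controlled character.
; The IA_InfoSetter input toggles the open menu's visibility through FlipFlops, giving the info setter priority.
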(event Custom|ShowBuyHouse
  (params (houseSlot :type BP%20House%20Slot%20Object%20Reference))
  ;[1 1 1] Create / destroy buy house widget
  (Default|SRSetHouseSlot (.AsBP%20Third%20Person%20Character (Utilities|Casting|CastToBP_ThirdPersonCharacter (Pawn|GetControlledPawn))) houseSlot)
  (if (Pawn|IsLocalPlayerController)
    (bind _returnvalue (UserInterface|CreateWidget "/Game/Game/Empire/UI/WBP_BuyHouse.WBP_BuyHouse_C"))
    (bind _output_get (Variables|Default|SetbuyHouseWidgetRef _returnvalue))
    (UserInterface|Viewport|AddtoViewport _output_get 0)
    (Variables|Default|SetisInBuyHouse true)))

(event Custom|HideBuyHouse
  (bind _buyhousewidgetref (Variables|Default|GetbuyHouseWidgetRef))
  ;[1 1 1] Create / destroy buy house widget
  (Default|SRSetHouseSlot (.AsBP%20Third%20Person%20Character (Utilities|Casting|CastToBP_ThirdPersonCharacter (Pawn|GetControlledPawn))))
  (if (Pawn|IsLocalPlayerController)
    (Utilities|IsValid _buyhousewidgetref
      (:Is%20Valid
        (Widget|RemovefromParent _buyhousewidgetref)
        (Variables|Default|SetisInBuyHouse false)
        (Default|ChangeLeaveVisibility (Variables|Default|GetbaseHudRef) false)))))

(event Custom|ShowInfoSetterWidget
  ;[1 1 1] Create / destroy player info setter widget
  (if (Pawn|IsLocalPlayerController)
    (bind _returnvalue (UserInterface|CreateWidget "/Game/Game/Empire/UI/WBP_PlayerInfosSetter.WBP_PlayerInfosSetter_C"))
    (bind _output_get (Variables|Default|SetplayerInfoSetterRef _returnvalue))
    (UserInterface|Viewport|AddtoViewport _output_get 0)
    (Variables|Default|SetisInInfoSetter true)))

(event Custom|HideInfoSetterWidget
  (bind _playerinfosetterref (Variables|Default|GetplayerInfoSetterRef))
  ;[1 1 1] Create / destroy player info setter widget
  (if (Pawn|IsLocalPlayerController)
    (Utilities|IsValid _playerinfosetterref
      (:Is%20Valid
        (Widget|RemovefromParent _playerinfosetterref)
        (Variables|Default|SetisInInfoSetter false)))))

(event Input|EnhancedActionEvents|EnhancedInputActionIA_InfoSetter
  (params (ActionValue :type Boolean) (ElapsedSeconds :type Float%20%28double-precision%29) (TriggeredSeconds :type Float%20%28double-precision%29) (InputAction :type Input%20Action%20Object%20Reference :default "/Game/ThirdPerson/Input/Actions/IA_InfoSetter.IA_InfoSetter"))
  (bind _playerinfosetterref (Variables|Default|GetplayerInfoSetterRef))
  (bind _buyhousewidgetref (Variables|Default|GetbuyHouseWidgetRef))
  ;[1 1 1] Show the menu (buy house / player info setter)
  (:Started
    (if (Pawn|IsLocalPlayerController)
      (if (Variables|Default|GetisInInfoSetter)
        (Utilities|FlowControl|FlipFlop ; Flip flop is not the best option
          (:A
            (Default|ChangeInfoSetterVisibility _playerinfosetterref true))
          (:B
            (Default|ChangeInfoSetterVisibility _playerinfosetterref false)))
        (elif (Variables|Default|GetisInBuyHouse)
          (Utilities|FlowControl|FlipFlop ; here it's not the best option aswell
            (:A
              (Default|ChangeBuyHouseVisibility _buyhousewidgetref true))
            (:B
              (Default|ChangeBuyHouseVisibility _buyhousewidgetref false))))))))

(event EventBeginPlay
  ;[1 1 1] Begin play, create player main hud
  (if (Pawn|IsLocalPlayerController)
    (bind _returnvalue (UserInterface|CreateWidget "/Game/Game/Empire/UI/WBP_PlayerBaseHud.WBP_PlayerBaseHud_C"))
    (bind _output_get (Variables|Default|SetbaseHudRef _returnvalue))
    (UserInterface|Viewport|AddtoViewport _output_get 0)))

(fn ConstructionScript)